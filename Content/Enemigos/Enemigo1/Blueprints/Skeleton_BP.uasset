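; Skeleton enemy character that runs a behavior tree, fights with a spawned right-hand weapon and supports player lock-on.
; Sight, damage and the player leaving its sphere update a behaviour enum mirrored to the Blackboard.
; Random attack montages pair with a trace component referencing the weapon, while a rotate component targets the player.
; Random level sets health; hits update its bar and play reactions, and death stops AI, releases lock-on and destroys it.
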(event `self.ReceiveBeginPlay`
  (bind _returnvalue (`KismetMathLibrary.RandomIntegerInRange` (`self.Nivel`) 3))
  ;[1 1 1] Arma Mano Derecha Spawn
  (`AIController.RunBehaviorTree` (`AIBlueprintHelperLibrary.GetAIController` self) "/Game/Enemigos/Enemigo1/BehaviourTree/Skeleton_BT.Skeleton_BT")
  (bind _returnvalue_2 (`|SpawnActorFromClass` (`self.ArmaDerechaPrueba`) (`SceneComponent.GetSocketTransform` (`self.Mesh`) "ArmaDerecha" "RTS_World") "Undefined" "OverrideRootScale" null null))
  (bind _output_get (set `self.ArmaDerechaActual` _returnvalue_2))
  (`self.K2_AttachToComponent` _output_get (`self.Mesh`) "ArmaDerecha" "SnapToTarget" "SnapToTarget" "SnapToTarget" true)
  (set `/Game/Equipment/BPC_TraceComponent.SwordRef` (`self.ArmaDerechaActual`) (`self.BCP_TraceComponent`))
  (bind _asbp_third_person_character (cast `/Game/ThirdPerson/Blueprints/BP_ThirdPersonCharacter` (`GameplayStatics.GetPlayerCharacter` 0)))
  (set `self.PlayerRef` _asbp_third_person_character)
  ;[1 1 1] Behaviour ENUM
  (`BlackboardComponent.SetValueAsEnum` (`AIBlueprintHelperLibrary.GetBlackboard` null) "ebehaviour" (`self.Behaviour`))
  (set `/Game/Equipment/BPC_RotateComponent.Target` (`GameplayStatics.GetPlayerCharacter` 0) (`self.BCP_RotateComponent`))
  (bind _outactors (`GameplayStatics.GetAllActorsWithTag` "Enemy"))
  (set `/Game/Equipment/BPC_TraceComponent.Enemy` _outactors (`self.BCP_TraceComponent`))
  (set `self.Nivel` _returnvalue)
  (bind _output_get_2 (set `self.Salud` (`KismetMathLibrary.Conv_IntToDouble` (* _returnvalue 20))))
  (set `self.SaludMaxima` _output_get_2)
  (bind _aswb_enemigo_1_salud (cast `/Game/Enemigos/Enemigo1/Widgets/WB_Enemigo1_Salud` (`WidgetComponent.GetWidget` (`self.SaludBar`))))
  (bind _output_get_3 (set `self.WB_SaludREF` _aswb_enemigo_1_salud))
  (set `/Game/Enemigos/Enemigo1/Widgets/WB_Enemigo1_Salud.SkeletonBP` self _output_get_3))

(event `self.ReceiveAnyDamage`
  (params (Damage :type "Float (single-precision)") (DamageType :type "DamageType Object Reference") (InstigatedBy :type "Controller Object Reference") (DamageCauser :type "Actor Object Reference"))
  (bind _targetactor (`/Game/ThirdPerson/Blueprints/BP_ThirdPersonCharacter.TargetActor` (`self.PlayerRef`)))
  ;[1 1 1] Damage System
  (set `self.Behaviour` "NewEnumerator3")
  (`BlackboardComponent.SetValueAsEnum` (`AIBlueprintHelperLibrary.GetBlackboard` null) "ebehaviour" (`self.Behaviour`))
  (set `self.Salud` (- (`self.Salud`) Damage))
  (if (<= (`self.Salud`) 0.0)
    (`/Engine/EditorBlueprintResources/StandardMacros.DoOnce` false
      (:`Completed`
        (`PrimitiveComponent.SetCollisionEnabled` (`self.CapsuleComponent`) "NoCollision")
        (`SceneComponent.SetVisibility` (`self.SaludBar`) false false)
        (`BrainComponent.StopLogic` (`AIController.BrainComponent` (`AIBlueprintHelperLibrary.GetAIController` self)) "die")
        (set `self.Muerto?` true)
        (`self.PlayAnimMontage` "/Game/Enemigos/Enemigo1/Animaciones/SkeleDeath_Montage.SkeleDeath_Montage")
        (`/Engine/EditorBlueprintResources/StandardMacros.IsValid` _targetactor
          (:`Is Valid`
            (if (== _targetactor self)
              (`/Game/ThirdPerson/Blueprints/BP_ThirdPersonCharacter.DisengagedLockOn` (`self.PlayerRef`))))
          (:`Is Not Valid`
            _))
        (`KismetSystemLibrary.Delay` 5.0)
        (`self.K2_DestroyActor`)))
    (else
      (`SceneComponent.SetVisibility` (`self.SaludBar`) true false)
      (`/Game/Enemigos/Enemigo1/Widgets/WB_Enemigo1_Salud.UpdateSaludBar` (`self.WB_SaludREF`))
      (`MovementComponent.StopMovementImmediately` (`self.CharacterMovement`))
      (bind _returnvalue (`self.PlayAnimMontage` "/Game/Enemigos/Enemigo1/Animaciones/Skele_Hit_Montage.Skele_Hit_Montage"))
      (`KismetSystemLibrary.RetriggerableDelay` _returnvalue)
      (set `self.Behaviour` "NewEnumerator3")
      (`BlackboardComponent.SetValueAsEnum` (`AIBlueprintHelperLibrary.GetBlackboard` null) "ebehaviour" (`self.Behaviour`)))))

(event `/Game/LockON/LockOnInterface.onSelected`
  ;[1 1 1] Visibility Focus
  (`SceneComponent.SetVisibility` (`self.BW_LockOn`) true false))

(event `/Game/LockON/LockOnInterface.onDeSelected`
  ;[1 1 1] Visibility Focus
  (`SceneComponent.SetVisibility` (`self.BW_LockOn`) false false))

(event `Attack`
  ;[1 1 1] Attack
  (bind _returnvalue (`self.PlayAnimMontage` (`KismetArrayLibrary.Array_Random` (`self.AttackAnimations`))))
  (set `self.AttackLength` _returnvalue))

(event `self.PawnSensing.OnSeePawn`
  (params (Pawn :type "Pawn Object Reference"))
  ;[1 1 1] Handle Enemy Vision
  (if (and (== Pawn (`GameplayStatics.GetPlayerCharacter` 0)) (`|EnumInequality` (`self.Behaviour`) "NewEnumerator0"))
    (set `self.Behaviour` "NewEnumerator3")
    (`BlackboardComponent.SetValueAsEnum` (`AIBlueprintHelperLibrary.GetBlackboard` null) "ebehaviour" (`self.Behaviour`))))

(event `self.Sphere.OnComponentEndOverlap`
  (params (OverlappedComponent :type "PrimitiveComponent Object Reference") (OtherActor :type "Actor Object Reference") (OtherComp :type "PrimitiveComponent Object Reference") (OtherBodyIndex :type Integer))
  ;[1 1 1] Scape Enemy
  (cast `/Game/ThirdPerson/Blueprints/BP_ThirdPersonCharacter` OtherActor)
  (if (not (`self.Muerto?`))
    (set `self.Behaviour` "NewEnumerator1")
    (`BlackboardComponent.SetValueAsEnum` (`AIBlueprintHelperLibrary.GetBlackboard` null) "ebehaviour" (`self.Behaviour`))
    (`SceneComponent.SetVisibility` (`self.SaludBar`) false false)))

(event `ClearHitActors`
  (`KismetArrayLibrary.Array_Clear` (`/Game/Equipment/BPC_TraceComponent.ActorsToIgnore` (`self.BCP_TraceComponent`))))

(fn `isDead`
  (returns (`isDead?` :type Boolean))
  (return (`self.Muerto?`)))

(fn `UserConstructionScript`)