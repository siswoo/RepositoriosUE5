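; Boss enemy Blueprint that runs the BT_Boss1 behavior tree and fights the player with melee and projectile attacks.
; BeginPlay attaches a weapon to the hand socket, feeds it to the trace component, targets the player for rotation and derives health from level.
; Random-rate montages drive attacks, storing their lengths; FireProjectile spawns shots aimed at the player.
; Damage updates the health bar widget; death stops AI, collision and movement; selection toggles a lock-on marker.
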(event `self.ReceiveBeginPlay`
  (bind _returnvalue (* (`self.Nivel`) 10))
  (`AIController.RunBehaviorTree` (`AIBlueprintHelperLibrary.GetAIController` self) "/Game/Enemigos/Enemigo2/BehaviourTree/BT_Boss1.BT_Boss1")
  (bind _returnvalue_2 (`|SpawnActorFromClass` (`self.Arma1Ref`) (`SceneComponent.GetSocketTransform` (`self.Mesh`) "ArmaDerecha" "RTS_World") "Undefined" "OverrideRootScale" null null))
  (bind _output_get (set `self.ArmaDerechaActual` _returnvalue_2))
  (`self.K2_AttachToComponent` _output_get (`self.Mesh`) "ArmaDerecha" "SnapToTarget" "SnapToTarget" "SnapToTarget" true)
  (set `/Game/Equipment/BPC_TraceComponent.SwordRef` (`self.ArmaDerechaActual`) (`self.BCP_TraceComponent`))
  (bind _asbp_third_person_character (cast `/Game/ThirdPerson/Blueprints/BP_ThirdPersonCharacter` (`GameplayStatics.GetPlayerCharacter` 0)))
  (set `self.PlayerRef` _asbp_third_person_character)
  ;[1 1 1] Behaviour ENUM
  (`BlackboardComponent.SetValueAsEnum` (`AIBlueprintHelperLibrary.GetBlackboard` null) "ebehaviour" (`self.Behaviour`))
  (set `/Game/Equipment/BPC_RotateComponent.Target` (`GameplayStatics.GetPlayerCharacter` 0) (`self.BCP_RotateComponent`))
  (bind _outactors (`GameplayStatics.GetAllActorsWithTag` "Enemy"))
  (set `/Game/Equipment/BPC_TraceComponent.Enemy` _outactors (`self.BCP_TraceComponent`))
  (set `self.Nivel` _returnvalue)
  (bind _output_get_2 (set `self.Salud` (`KismetMathLibrary.Conv_IntToDouble` (* _returnvalue 20))))
  (set `self.SaludMaxima` _output_get_2)
  (bind _aswb_boss_salud (cast `/Game/Enemigos/Enemigo2/Widgets/WB_Boss_Salud` (`WidgetComponent.GetWidget` (`self.SaludBar`))))
  (bind _output_get_3 (set `self.WB_BossSalud` _aswb_boss_salud))
  (set `/Game/Enemigos/Enemigo2/Widgets/WB_Boss_Salud.Boss1Ref` self _output_get_3))

(event `self.ReceiveAnyDamage`
  (params (Damage :type "Float (single-precision)") (DamageType :type "DamageType Object Reference") (InstigatedBy :type "Controller Object Reference") (DamageCauser :type "Actor Object Reference"))
  ;[1 1 1] Damage System
  (bind _output_get (set `self.Salud` (- (`self.Salud`) Damage)))
  (if (<= _output_get 0.0)
    (set `self.Salud` 0.0)
    (`/Engine/EditorBlueprintResources/StandardMacros.DoOnce` false
      (:`Completed`
        (`BrainComponent.StopLogic` (`AIController.BrainComponent` (`AIBlueprintHelperLibrary.GetAIController` self)) "")
        (`self.PlayAnimMontage` "/Game/Enemigos/Enemigo2/Animaciones/ExoGame_Troll_Death__Montage.ExoGame_Troll_Death__Montage")
        (`PrimitiveComponent.SetCollisionEnabled` (`self.CapsuleComponent`) "NoCollision")
        (`ActorComponent.K2_DestroyComponent` (`self.CharacterMovement`))
        (`Widget.RemoveFromParent` (`self.WB_BossSalud`))
        (`SceneComponent.SetVisibility` (`self.SaludBar`) false false)
        (`/Game/Enemigos/Enemigo2/Widgets/WB_Boss_Salud.UpdateSaludBar` (`self.WB_BossSalud`))))
    (else
      (`SceneComponent.SetVisibility` (`self.SaludBar`) true false)
      (`/Game/Enemigos/Enemigo2/Widgets/WB_Boss_Salud.UpdateSaludBar` (`self.WB_BossSalud`)))))

(event `/Game/LockON/LockOnInterface.onSelected`
  ;[1 1 1] Visibility Focus
  (`SceneComponent.SetVisibility` (`self.BW_LockOn`) true false))

(event `/Game/LockON/LockOnInterface.onDeSelected`
  ;[1 1 1] Visibility Focus
  (`SceneComponent.SetVisibility` (`self.BW_LockOn`) false false))

(event `Attack`
  ;[1 1 1] Attack Melee
  (bind _returnvalue (`self.PlayAnimMontage` (`KismetArrayLibrary.Array_Random` (`self.AttackAnimations`)) (`KismetMathLibrary.Conv_IntToDouble` (`KismetMathLibrary.RandomIntegerInRange` 1 2))))
  (set `self.AttackLength` _returnvalue))

(event `ClearHitActors`
  ;[1 1 1] ClearActorHit
  (`KismetArrayLibrary.Array_Clear` (`/Game/Equipment/BPC_TraceComponent.ActorsToIgnore` (`self.BCP_TraceComponent`))))

(event `ProjectileAttack1`
  ;[1 1 1] Projectile Attack
  (bind _returnvalue (`self.PlayAnimMontage` "/Game/InfinityBladeAdversaries/Enemy/Enemy_Troll/Enemy_Troll_Poison_Animation/Boss1ProjectileAttack.Boss1ProjectileAttack" (`KismetMathLibrary.Conv_IntToDouble` (`KismetMathLibrary.RandomIntegerInRange` 1 2))))
  (set `self.RangeAttackLength` _returnvalue))

(event `FireProjectile`
  (bind _returnvalue (`SceneComponent.K2_GetComponentLocation` (`self.ProjectileSpawnPoint`)))
  ;[1 1 1] Efect Fire Projectile Attack
  (`|SpawnActorFromClass` "/Game/Enemigos/Enemigo2/Boss1Projectile1_BP.Boss1Projectile1_BP_C" (`KismetMathLibrary.MakeTransform` _returnvalue (`KismetMathLibrary.FindLookAtRotation` _returnvalue (`self.K2_GetActorLocation` (`GameplayStatics.GetPlayerCharacter` 0)))) "Undefined" "OverrideRootScale" null null))

(fn `isDead`
  (returns (`isDead?` :type Boolean))
  (return (`self.Muerto?`)))

(fn `UserConstructionScript`)