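; Actor component that handles sword hit detection and damage for melee attacks.
; While the weapon is active, each tick sphere-traces for Pawns between the sword mesh's Start and End sockets, ignoring Enemy.
; New hits take sword damage plus the player character's PoderDeAtaque stat and spawn a blood splat.
; Hit actors join an ignore list, preventing repeat damage; this graph never clears it.
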(event `self.ReceiveTick`
  (params (DeltaSeconds :type "Float (single-precision)"))
  (bind _asbp_third_person_character (cast `/Game/ThirdPerson/Blueprints/BP_ThirdPersonCharacter` (`GameplayStatics.GetPlayerCharacter` 0)))
  (set `self.Player` _asbp_third_person_character)
  (if (`self.WeaponActive?`)
    (bind _outhits (`KismetSystemLibrary.SphereTraceMultiForObjects` (`SceneComponent.GetSocketLocation` (`/Game/Equipment/Swords/01/Sword1_BP.SkeletalMesh` (`self.SwordRef`)) "Start") (`SceneComponent.GetSocketLocation` (`/Game/Equipment/Swords/01/Sword1_BP.SkeletalMesh` (`self.SwordRef`)) "End") (`/Game/Equipment/Swords/01/Sword1_BP.TraceSize` (`self.SwordRef`)) (`|MakeArray` "ObjectTypeQuery3" :!type "EObjectTypeQuery Enum") false (`self.Enemy`) "None" true (struct :`R` 0.184225 :`G` 1.0 :`A` 1.0) (struct :`R` 0.4375 :`B` 0.009015 :`A` 1.0) 2.0))
    (for _array_element _outhits
      (bind (_bblockinghit _binitialoverlap _time _distance _location _impactpoint _normal _impactnormal _physmat _hitactor) (`GameplayStatics.BreakHitResult` _array_element))
      (if (not (`KismetArrayLibrary.Array_Contains` (`self.ActorsToIgnore`) _hitactor))
        (`GameplayStatics.ApplyDamage` _hitactor (+ (`/Game/Equipment/Swords/01/Sword1_BP.Damage` (`self.SwordRef`)) (`/Game/PlayerStatus/BPC_PlayerStatus.PoderDeAtaque` (`/Game/ThirdPerson/Blueprints/BP_ThirdPersonCharacter.BPC_PlayerStatus` (`self.Player`)))) null (`self.GetOwner`))
        (`KismetArrayLibrary.Array_Add` (`self.ActorsToIgnore`) _hitactor)
        (`GameplayStatics.SpawnEmitterAtLocation` "/Game/Realistic_Starter_VFX_Pack_Vol2/Particles/Blood/P_Blood_Splat_Cone.P_Blood_Splat_Cone" _location (`KismetMathLibrary.MakeRotFromZ` _location))))))