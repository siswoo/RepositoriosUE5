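; BPC_RotateComponent is an actor component that turns its owning actor to face a Target actor while Shouldrotate is true.
; Each Tick it computes the look-at rotation from owner to Target and moves only the yaw toward it at a constant rate, preserving pitch and roll.
; The interpolation treats yaw as a plain float, so it does not take the shortest path across the ±180 degree wrap.
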(event `self.ReceiveTick`
  (params (DeltaSeconds :type "Float (single-precision)"))
  (bind _returnvalue (`self.GetOwner`))
  (bind (_returnvalue_roll _returnvalue_pitch _returnvalue_yaw) (`KismetMathLibrary.BreakRotator` (`Actor.K2_GetActorRotation` _returnvalue)))
  (bind (_returnvalue_roll_2 _returnvalue_pitch_2 _returnvalue_yaw_2) (`KismetMathLibrary.BreakRotator` (`KismetMathLibrary.FindLookAtRotation` (`Actor.K2_GetActorLocation` _returnvalue) (`Actor.K2_GetActorLocation` (`self.Target`)))))
  (if (`self.shouldrotate?`)
    (`Actor.K2_SetActorRotation` _returnvalue (`KismetMathLibrary.MakeRotator` _returnvalue_roll _returnvalue_pitch (`KismetMathLibrary.FInterpTo_Constant` _returnvalue_yaw _returnvalue_yaw_2 (`GameplayStatics.GetWorldDeltaSeconds`) 300.0)) false)))