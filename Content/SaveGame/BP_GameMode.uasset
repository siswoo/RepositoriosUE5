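; Game mode that exposes save, load and restart events for a single save slot holding the player character's transform.
; Saving writes that transform into an existing BP_SaveGame and stops if the cast fails.
; Loading only restarts the level; restarting also deletes the slot first.
; The logic that would create the save or restore the transform is unconnected and never runs, with BeginPlay empty.
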(event `self.ReceiveBeginPlay`)

(event `Save Game`
  ;[1 1 1] Save Game
  (bind _returnvalue (`GameplayStatics.LoadGameFromSlot` "Save1"))
  (bind _asbp_save_game (cast `/Game/SaveGame/BP_SaveGame` _returnvalue))
  (set `/Game/SaveGame/BP_SaveGame.CharTransform` (`self.GetTransform` (cast `/Game/ThirdPerson/Blueprints/BP_ThirdPersonCharacter` (`GameplayStatics.GetPlayerCharacter` 0) :!pure true)) _asbp_save_game)
  (`GameplayStatics.SaveGameToSlot` _asbp_save_game "Save1"))

(event `LoadGame`
  ;[1 1 1] LoadGame
  (`KismetSystemLibrary.ExecuteConsoleCommand` "RestartLevel" null))

(event `RestartLevel`
  ;[1 1 1] Delete Save + Restart
  (`GameplayStatics.DeleteGameInSlot` "Save1")
  (`KismetSystemLibrary.ExecuteConsoleCommand` "RestartLevel" null))

(fn `UserConstructionScript`)