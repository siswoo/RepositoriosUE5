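; Ladrillo NPC Blueprint that shows its name text and a quest widget while something overlaps its interaction box.
; Overlap events set an in-range flag and toggle both displays through MostrarOcultarQuest and RotateText.
; RotateText re-calls itself after a short Delay while in range, turning the name toward the player and setting the widget's relative rotation from the player's.
; The mission-chain function CadenaDeMision is an empty stub.
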(event `self.ReceiveBeginPlay`
  (bind _asbp_third_person_character (cast `/Game/ThirdPerson/Blueprints/BP_ThirdPersonCharacter` (`GameplayStatics.GetPlayerCharacter` 0)))
  (set `self.Player` _asbp_third_person_character)
  (`TextRenderComponent.K2_SetText` (`self.TextRender`) (`KismetTextLibrary.Conv_NameToText` (`self.Nombre`))))

(event `self.Box.OnComponentBeginOverlap`
  (params (OverlappedComponent :type "PrimitiveComponent Object Reference") (OtherActor :type "Actor Object Reference") (OtherComp :type "PrimitiveComponent Object Reference") (OtherBodyIndex :type Integer) (bFromSweep :type Boolean) (SweepResult :type "HitResult Structure (by ref)"))
  (`self.Mostrar/Ocultar Quest` true)
  (set `self.CampoDeInteraccion?` true)
  (`self.RotateText` true))

(event `self.Box.OnComponentEndOverlap`
  (params (OverlappedComponent :type "PrimitiveComponent Object Reference") (OtherActor :type "Actor Object Reference") (OtherComp :type "PrimitiveComponent Object Reference") (OtherBodyIndex :type Integer))
  (`self.Mostrar/Ocultar Quest` false)
  (set `self.CampoDeInteraccion?` false)
  (`self.RotateText` false))

(event `RotateText`
  (params (`On?` :type Boolean))
  (bind (_returnvalue_roll _returnvalue_pitch _returnvalue_yaw) (`KismetMathLibrary.BreakRotator` (`KismetMathLibrary.FindLookAtRotation` (`self.K2_GetActorLocation`) (`self.K2_GetActorLocation` (`self.Player`)))))
  ;[1 1 1] Rotate Text Widget
  (if `On?`
    (`SceneComponent.SetVisibility` (`self.TextRender`) true false)
    (`SceneComponent.K2_SetWorldRotation` (`self.TextRender`) (`KismetMathLibrary.MakeRotator` 0.0 _returnvalue_pitch _returnvalue_yaw) false false)
    (`SceneComponent.K2_SetRelativeRotation` (`self.Widget`) (`self.K2_GetActorRotation` (`self.Player`)) false false)
    (`KismetSystemLibrary.Delay` 0.01)
    (if (`self.CampoDeInteraccion?`)
      (`self.RotateText` true)
      (else
        (`self.RotateText` false)))
    (else
      (`SceneComponent.SetVisibility` (`self.TextRender`) false false))))

(fn `CadenaDeMision`
  (params (NivelRequerido :type Integer) (Cadena :type Integer) (NPC :type Name)))

(fn `Mostrar/Ocultar Quest`
  (params (`Mostrar?` :type Boolean))
  (if `Mostrar?`
    (`SceneComponent.SetVisibility` (`self.Widget`) true false)
    (`self.RotateText` true)
    (else
      (`SceneComponent.SetVisibility` (`self.Widget`) false false)
      (`self.RotateText` false))))

(fn `UserConstructionScript`)