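; Player status component for BP_ThirdPersonCharacter that tracks health, mana, energy, experience and level.
; Incrementa and Disminuye apply one amount to flag-selected stats through chained macros; only Incrementa handles experience, and several flags are unused.
; Stat macros clamp health, mana and energy, flag death at zero health and level up at Nivel × 35 experience.
; Each change refreshes its bar in the player's MenuHUDStatus widget.
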(event `self.ReceiveBeginPlay`
  (bind _asbp_third_person_character (cast `/Game/ThirdPerson/Blueprints/BP_ThirdPersonCharacter` (`self.GetOwner`)))
  (set `self.PlayerRef` _asbp_third_person_character))

(fn `Disminuye`
  (params (`Salud?` :type Boolean) (`Mana?` :type Boolean) (`Energia?` :type Boolean) (`Alteracion?` :type Boolean) (`Nivel?` :type Boolean) (`Velocidades?` :type Boolean) (`Resistencias?` :type Boolean) (`Perks?` :type Boolean) (Cantidad :type "Float (double-precision)"))
  (`self.MSalud` `Salud?` false Cantidad
    (:`Out`
      (`self.MMana` `Mana?` false Cantidad
        (:`Out`
          (`self.MEnergia` `Energia?` false Cantidad
            (:`Out`
              (return))))))))

(fn `Incrementa`
  (params (`Salud?` :type Boolean) (`Mana?` :type Boolean) (`Energia?` :type Boolean) (`Alteracion?` :type Boolean) (`Nivel?` :type Boolean) (`Velocidades?` :type Boolean) (`Resistencias?` :type Boolean) (`Perks?` :type Boolean) (Cantidad :type "Float (double-precision)"))
  (`self.MSalud` `Salud?` true Cantidad
    (:`Out`
      (`self.MMana` `Mana?` true Cantidad
        (:`Out`
          (`self.MEnergia` `Energia?` true Cantidad
            (:`Out`
              (`self.MNivel` `Nivel?` true Cantidad
                (:`Out`
                  (return))))))))))

(fn `Update WB HUD`
  (params (`Salud?` :type Boolean) (`Mana?` :type Boolean) (`Energia?` :type Boolean) (`Experiencia?` :type Boolean) (`Nivel?` :type Boolean) (Cantidad :type "Float (double-precision)"))
  (`self.WBSalud` `Salud?`))