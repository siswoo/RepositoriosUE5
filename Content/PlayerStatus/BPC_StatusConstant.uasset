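; Actor component on BP_ThirdPersonCharacter that passively regenerates the player's health, mana and energy.
; On BeginPlay it caches the owner's BPCPlayerStatus and, after a short delay, starts three looping timers, one per stat.
; Each tick of a timer adds that stat's regeneration rate, carrying the fractional remainder between cycles so only whole points are applied.
; Values clamp at their maximum, and each update refreshes the HUD through BPCPlayerStatus.
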(event `self.ReceiveBeginPlay`
  (bind _asbp_third_person_character (cast `/Game/ThirdPerson/Blueprints/BP_ThirdPersonCharacter` (`self.GetOwner`)))
  (bind _output_get (set `self.PlayerRef` _asbp_third_person_character))
  (set `self.PlayerStatusRef` (`/Game/ThirdPerson/Blueprints/BP_ThirdPersonCharacter.BPC_PlayerStatus` _output_get))
  (`KismetSystemLibrary.Delay` 0.2)
  (`KismetSystemLibrary.K2_SetTimer` null "RegeSalud" 3.0 true)
  (`KismetSystemLibrary.K2_SetTimer` null "RegeMana" 3.0 true)
  (`KismetSystemLibrary.K2_SetTimer` null "RegeEnergia" 3.0 true))

(event `self.ReceiveTick`
  (params (DeltaSeconds :type "Float (single-precision)")))

(fn `RegeEnergia`
  (bind _playerstatusref (`self.PlayerStatusRef`))
  (bind _playerstatusref_2 (`self.PlayerStatusRef`))
  (bind _output_get (set `self.EnergiaEstancada` (+ (`/Game/PlayerStatus/BPC_PlayerStatus.RegeneracionEnergia` (`self.PlayerStatusRef`)) (`self.EnergiaEstancada`))))
  (set `/Game/PlayerStatus/BPC_PlayerStatus.Energia` (+ (`/Game/PlayerStatus/BPC_PlayerStatus.Energia` (`self.PlayerStatusRef`)) (`KismetMathLibrary.FTrunc` _output_get)) (`self.PlayerStatusRef`))
  (if (>= (`/Game/PlayerStatus/BPC_PlayerStatus.Energia` _playerstatusref_2) (`/Game/PlayerStatus/BPC_PlayerStatus.Energia_Maxima` _playerstatusref_2))
    (set `/Game/PlayerStatus/BPC_PlayerStatus.Energia` (`/Game/PlayerStatus/BPC_PlayerStatus.Energia_Maxima` _playerstatusref) _playerstatusref)
    (set `self.EnergiaEstancada` 0.0)
    (else
      (set `self.EnergiaEstancada` (`KismetMathLibrary.Fraction` (`self.EnergiaEstancada`)))))
  (`/Game/PlayerStatus/BPC_PlayerStatus.Update WB HUD` (`self.PlayerStatusRef`) false false true false false 0.0)
  (return))

(fn `RegeMana`
  (bind _playerstatusref (`self.PlayerStatusRef`))
  (bind _playerstatusref_2 (`self.PlayerStatusRef`))
  (bind _output_get (set `self.ManaEstancada` (+ (`/Game/PlayerStatus/BPC_PlayerStatus.RegeneracionMana` (`self.PlayerStatusRef`)) (`self.ManaEstancada`))))
  (set `/Game/PlayerStatus/BPC_PlayerStatus.Mana` (+ (`/Game/PlayerStatus/BPC_PlayerStatus.Mana` (`self.PlayerStatusRef`)) (`KismetMathLibrary.FTrunc` _output_get)) (`self.PlayerStatusRef`))
  (if (>= (`/Game/PlayerStatus/BPC_PlayerStatus.Mana` _playerstatusref_2) (`/Game/PlayerStatus/BPC_PlayerStatus.Mana_Maxima` _playerstatusref_2))
    (set `/Game/PlayerStatus/BPC_PlayerStatus.Mana` (`/Game/PlayerStatus/BPC_PlayerStatus.Mana_Maxima` _playerstatusref) _playerstatusref)
    (set `self.ManaEstancada` 0.0)
    (else
      (set `self.ManaEstancada` (`KismetMathLibrary.Fraction` (`self.ManaEstancada`)))))
  (`/Game/PlayerStatus/BPC_PlayerStatus.Update WB HUD` (`self.PlayerStatusRef`) false true false false false 0.0)
  (return))

(fn `RegeSalud`
  (bind _playerstatusref (`self.PlayerStatusRef`))
  (bind _playerstatusref_2 (`self.PlayerStatusRef`))
  (bind _output_get (set `self.SaludEstancada` (+ (`/Game/PlayerStatus/BPC_PlayerStatus.RegeneracionSalud` (`self.PlayerStatusRef`)) (`self.SaludEstancada`))))
  (set `/Game/PlayerStatus/BPC_PlayerStatus.Salud` (+ (`/Game/PlayerStatus/BPC_PlayerStatus.Salud` (`self.PlayerStatusRef`)) (`KismetMathLibrary.FTrunc` _output_get)) (`self.PlayerStatusRef`))
  (if (>= (`/Game/PlayerStatus/BPC_PlayerStatus.Salud` _playerstatusref_2) (`/Game/PlayerStatus/BPC_PlayerStatus.Salud_Maxima` _playerstatusref_2))
    (set `/Game/PlayerStatus/BPC_PlayerStatus.Salud` (`/Game/PlayerStatus/BPC_PlayerStatus.Salud_Maxima` _playerstatusref) _playerstatusref)
    (set `self.SaludEstancada` 0.0)
    (else
      (set `self.SaludEstancada` (`KismetMathLibrary.Fraction` (`self.SaludEstancada`)))))
  (`/Game/PlayerStatus/BPC_PlayerStatus.Update WB HUD` (`self.PlayerStatusRef`) true false false false false 0.0)
  (return))